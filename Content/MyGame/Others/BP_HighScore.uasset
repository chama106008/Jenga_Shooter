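; BP_HighScore stores per-stage high scores for the game and provides functions to update and reset them.
; UpdateHighScore switches on the stage ID and overwrites that stage's variable with the result of IsHighScore, which returns the higher of the new and stored scores rather than a boolean.
; ResetHighScore zeroes the scores for Worlds 1 to 3, though updates only handle Worlds 1 and 2.
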(fn UpdateHighScore
  (params (StageID :type Name) (NewScore :type Integer))
  (switch name StageID
    (:1-1
      ;[1 1 1] World1
      (bind _score (CallFunction|IsHighScore NewScore (Variables|Default|Get1-1)))
      (Variables|Default|Set1-1 _score))
    (:1-2
      (bind _score_2 (CallFunction|IsHighScore NewScore (Variables|Default|Get1-2)))
      (Variables|Default|Set1-2 _score_2))
    (:1-3
      (bind _score_3 (CallFunction|IsHighScore NewScore (Variables|Default|Get1-3)))
      (Variables|Default|Set1-3 _score_3))
    (:1-4
      (bind _score_4 (CallFunction|IsHighScore NewScore (Variables|Default|Get1-4)))
      (Variables|Default|Set1-4 _score_4))
    (:2-1
      ;[1 1 1] Wolrd2
      (bind _score_5 (CallFunction|IsHighScore NewScore (Variables|Default|Get2-1)))
      (Variables|Default|Set2-1 _score_5))
    (:2-2
      (bind _score_6 (CallFunction|IsHighScore NewScore (Variables|Default|Get2-2)))
      (Variables|Default|Set2-2 _score_6))
    (:2-3
      (bind _score_7 (CallFunction|IsHighScore NewScore (Variables|Default|Get2-3)))
      (Variables|Default|Set2-3 _score_7))
    (:2-4
      (bind _score_8 (CallFunction|IsHighScore NewScore (Variables|Default|Get2-4)))
      (Variables|Default|Set2-4 _score_8))))

(fn IsHighScore
  (params (NewScore :type Integer) (OldScore :type Integer))
  (if (> NewScore OldScore)
    (Variables|Default|Setreturnscore NewScore)
    (else
      (Variables|Default|Setreturnscore OldScore)))
  (return (Variables|Default|Getreturnscore)))

(fn ResetHighScore
  (Variables|Default|Set1-1 0)
  (Variables|Default|Set1-2 0)
  (Variables|Default|Set1-3 0)
  (Variables|Default|Set1-4 0)
  (Variables|Default|Set2-1 0)
  (Variables|Default|Set2-2 0)
  (Variables|Default|Set2-3 0)
  (Variables|Default|Set2-4 0)
  (Variables|Default|Set3-1 0)
  (Variables|Default|Set3-2 0)
  (Variables|Default|Set3-3 0)
  (Variables|Default|Set3-4 0))