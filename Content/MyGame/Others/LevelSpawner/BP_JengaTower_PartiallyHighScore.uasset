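; Jenga tower Blueprint variant that, going by its name, mixes higher-scoring blocks into the tower.
; Its only active logic is GetClass, which picks a block class from a layer and index.
; Index 1 gets MetalBlock when Layer % 1 is zero, which holds for any whole-number layer, and every other case gets WoodBlock.
; The event graph holds only disabled placeholder events.
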(event EventBeginPlay
  (|CallParentFunction) ; このノードは無効になっているため呼び出せません。\n機能をビルドするにはピンをドラッグしてください。
)

(event Collision|EventActorBeginOverlap
  (params (OtherActor :type Actor%20Object%20Reference))
  (|CallParentFunction OtherActor) ; このノードは無効になっているため呼び出せません。\n機能をビルドするにはピンをドラッグしてください。
)

(event EventTick
  (params (DeltaSeconds :type Float%20%28single-precision%29))
  (|CallParentFunction DeltaSeconds) ; このノードは無効になっているため呼び出せません。\n機能をビルドするにはピンをドラッグしてください。
)

(fn ConstructionScript
  (|CallParentFunction))

(fn GetClass
  (params (Layer :type Integer) (Index :type Integer))
  (if (== (Math|Integer|%(Integer) Layer 1) 0)
    (if (== Index 1)
      (Variables|Default|Setreturn%20class "/Game/MyGame/Objects/MetalBlock.MetalBlock_C")
      (else
        (Variables|Default|Setreturn%20class "/Game/MyGame/Objects/WoodBlock.WoodBlock_C" :!label _label)))
    (else
      (goto _label)))
  (return (Variables|Default|Getreturn%20class)))