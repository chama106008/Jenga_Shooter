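; Jenga tower level-spawner variant that decides which tower slots hold bomb blocks and which hold wood.
; GetClass returns a block class from layer and index, using an XOR of odd layer and index 1 to make an alternating pattern.
; Despite the AllBomb name, odd layers get bombs except at index 1, while even layers get a bomb only there.
; Events are disabled stubs, and construction only calls the parent.
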(event EventBeginPlay
  (|CallParentFunction) ; このノードは無効になっているため呼び出せません。\n機能をビルドするにはピンをドラッグしてください。
)

(event Collision|EventActorBeginOverlap
  (params (OtherActor :type Actor%20Object%20Reference))
  (|CallParentFunction OtherActor) ; このノードは無効になっているため呼び出せません。\n機能をビルドするにはピンをドラッグしてください。
)

(event EventTick
  (params (DeltaSeconds :type Float%20%28single-precision%29))
  (|CallParentFunction DeltaSeconds) ; このノードは無効になっているため呼び出せません。\n機能をビルドするにはピンをドラッグしてください。
)

(fn ConstructionScript
  (|CallParentFunction))

(fn GetClass
  (params (Layer :type Integer) (Index :type Integer))
  (if (Class|KismetMathLibrary|XORBoolean (== (Math|Integer|%(Integer) Layer 2) 1) (== Index 1))
    (Variables|Default|SetReturnClass "/Game/MyGame/Objects/BombBlock.BombBlock_C")
    (else
      (bind _output_get (Variables|Default|SetReturnClass "/Game/MyGame/Objects/WoodBlock.WoodBlock_C"))))
  (return _output_get))