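; Jenga tower spawner that builds a stack of block actors on BeginPlay.
; PlaceBlocks spawns three blocks per layer, switching the offset axis between X and Y and applying Rotation on alternate layers to form the criss-cross pattern.
; Spawn transforms are world-space around the origin, independent of the spawner's own transform.
; GetClass receives layer and slot as a hook for per-block selection, but here always returns DefaultBlockClass.
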(event EventBeginPlay
  (CallFunction|PlaceBlocks))

(event Collision|EventActorBeginOverlap
  (params (OtherActor :type Actor%20Object%20Reference)))

(event EventTick
  (params (DeltaSeconds :type Float%20%28single-precision%29)))

(fn ConstructionScript)

(fn PlaceBlocks
  (bind _rotation (Variables|Default|GetRotation))
  (bind _basescale (Variables|Default|GetBaseScale))
  (for _index (range 0 (- (Variables|Default|GetLayer) 1))
    (if (== (Math|Integer|%(Integer) _index 2) 1)
      ;[1 1 1] 偶数段目
      (bind _placeclass (CallFunction|GetClass (+ _index 1) 1))
      (Game|SpawnActorfromClass _placeclass (Math|Transform|MakeTransform (Math|Vector|MakeVector 0.0 0.0 (+ (* (Variables|Default|GetHeight) _index) 1e+02)) _rotation _basescale) "Undefined" "MultiplyWithRoot" 0 0)
      (bind _placeclass_2 (CallFunction|GetClass (+ _index 1) 2))
      (Game|SpawnActorfromClass _placeclass_2 (Math|Transform|MakeTransform (Math|Vector|MakeVector 2e+02 0.0 (+ (* (Variables|Default|GetHeight) _index) 1e+02)) _rotation _basescale) "Undefined" "MultiplyWithRoot" 0 0)
      (bind _placeclass_3 (CallFunction|GetClass (+ _index 1) 3))
      (Game|SpawnActorfromClass _placeclass_3 (Math|Transform|MakeTransform (Math|Vector|MakeVector -2e+02 0.0 (+ (* (Variables|Default|GetHeight) _index) 1e+02)) _rotation _basescale) "Undefined" "MultiplyWithRoot" 0 0)
      (else
        ;[1 1 1] 奇数段目
        (bind _placeclass_4 (CallFunction|GetClass (+ _index 1) 1))
        (Game|SpawnActorfromClass _placeclass_4 (Math|Transform|MakeTransform (Math|Vector|MakeVector 0.0 0.0 (+ (* (Variables|Default|GetHeight) _index) 1e+02)) "0, 0, 0" _basescale) "Undefined" "MultiplyWithRoot" 0 0)
        (bind _placeclass_5 (CallFunction|GetClass (+ _index 1) 2))
        (Game|SpawnActorfromClass _placeclass_5 (Math|Transform|MakeTransform (Math|Vector|MakeVector 0.0 2e+02 (+ (* (Variables|Default|GetHeight) _index) 1e+02)) "0, 0, 0" _basescale) "Undefined" "MultiplyWithRoot" 0 0)
        (bind _placeclass_6 (CallFunction|GetClass (+ _index 1) 3))
        (Game|SpawnActorfromClass _placeclass_6 (Math|Transform|MakeTransform (Math|Vector|MakeVector 0.0 -2e+02 (+ (* (Variables|Default|GetHeight) _index) 1e+02)) "0, 0, 0" _basescale) "Undefined" "MultiplyWithRoot" 0 0)))))

(fn GetClass
  (params (Layer :type Integer) (Index :type Integer))
  ;[1 1 1] 段数と配置（中央、右、左）に応じて設置するブロックを指定可能
  (return (Variables|Default|GetDefaultBlockClass)))