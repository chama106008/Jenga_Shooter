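; Jenga tower level-spawner Blueprint for what its name indicates is a high-score bomb layout.
; GetClass picks each block's class from its layer and index: index 1 gets a bomb on one specific layer and metal on other even layers, while every other position gets wood.
; The event graph holds only disabled default events, and the construction script just calls its parent.
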(event EventBeginPlay
  (|CallParentFunction) ; このノードは無効になっているため呼び出せません。\n機能をビルドするにはピンをドラッグしてください。
)

(event Collision|EventActorBeginOverlap
  (params (OtherActor :type Actor%20Object%20Reference))
  (|CallParentFunction OtherActor) ; このノードは無効になっているため呼び出せません。\n機能をビルドするにはピンをドラッグしてください。
)

(event EventTick
  (params (DeltaSeconds :type Float%20%28single-precision%29))
  (|CallParentFunction DeltaSeconds) ; このノードは無効になっているため呼び出せません。\n機能をビルドするにはピンをドラッグしてください。
)

(fn ConstructionScript
  (|CallParentFunction))

(fn 新規関数)

(fn GetClass
  (params (Layer :type Integer) (Index :type Integer))
  (if (== Index 1)
    (if (== Layer 8)
      (Variables|Default|SetReturnClass "/Game/MyGame/Objects/BombBlock.BombBlock_C")
      (elif (== (Math|Integer|%(Integer) Layer 2) 0)
        (Variables|Default|SetReturnClass "/Game/MyGame/Objects/MetalBlock.MetalBlock_C")
        (else
          (Variables|Default|SetReturnClass "/Game/MyGame/Objects/WoodBlock.WoodBlock_C" :!label _label))))
    (else
      (goto _label)))
  (return (Variables|Default|GetReturnClass)))