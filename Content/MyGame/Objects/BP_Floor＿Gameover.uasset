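; BP_Floor_Gameover is a fail-zone floor whose box overlap penalizes lost scorable objects and returns the player to the start.
; Actors implementing BPIScorable trigger fire and steam particles plus a fire sound at the player, are destroyed, and cost a life via LoseLife on BP_FirstPersonGameMode.
; Otherwise, an overlapping BP_FirstPersonCharacter is moved to the first PlayerStart found in the level.
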(event OnComponentBeginOverlap(Box)
  (params (OverlappedComponent :type Primitive%20Component%20Object%20Reference) (OtherActor :type Actor%20Object%20Reference) (OtherComp :type Primitive%20Component%20Object%20Reference) (OtherBodyIndex :type Integer) (bFromSweep :type Boolean) (SweepResult :type Hit%20Result%20Structure%20%28by%20ref%29))
  (bind _returnvalue (Transformation|GetWorldLocation OtherComp))
  ;[1 1 1] Scorableなら処理実行
  (if (Utilities|DoesObjectImplementInterface OtherActor "/Game/MyGame/Others/BPI＿Scorable.BPI＿Scorable_C")
    ;[1 1 1] 演出+処理
    (Effects|SpawnEmitteratLocation "/Game/StarterContent/Particles/P_Fire.P_Fire" _returnvalue "0, 0, 0" "20.000000,20.000000,30.000000" false)
    (Effects|SpawnEmitteratLocation "/Game/StarterContent/Particles/P_Steam_Lit.P_Steam_Lit" _returnvalue "0, 0, 0" "5.000000,5.000000,5.000000")
    (Audio|SpawnSoundatLocation "/Game/StarterContent/Audio/Fire01.Fire01" (Transformation|GetActorLocation (Game|GetPlayerCharacter 0)) "0, 0, 0" 3.0 1.0 0.0 0 0)
    (Actor|DestroyActor OtherActor)
    (bind _asbp_first_person_game_mode (Utilities|Casting|CastToBP_FirstPersonGameMode (Game|GetGameMode)))
    (Default|LoseLife _asbp_first_person_game_mode)
    (else
      ;[1 1 1] プレイヤーであれば初期地点に移動
      (bind _asbp_first_person_character (Utilities|Casting|CastToBP_FirstPersonCharacter OtherActor))
      (bind _outactors (Actor|GetAllActorsOfClass "/Script/Engine.PlayerStart"))
      (Transformation|SetActorLocation _asbp_first_person_character (Transformation|GetActorLocation (Utilities|Array|Get(acopy) _outactors)) false false))))

(event EventBeginPlay)

(event EventTick
  (params (DeltaSeconds :type Float%20%28single-precision%29)))

(fn ConstructionScript)