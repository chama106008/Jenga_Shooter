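; Level assembler actor that spawns a configured set of actors when play begins.
; PlaceActors pairs the PlaceClasses and PlaceTransforms arrays by index up to the shorter length, printing an error for any invalid class index.
; Each spawned actor is stored in SpawnedActors, which DestroyActors uses to remove them all and clear the list, though nothing in this Blueprint calls it.
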(event EventBeginPlay
  (CallFunction|PlaceActors))

(event Collision|EventActorBeginOverlap
  (params (OtherActor :type Actor%20Object%20Reference)))

(event EventTick
  (params (DeltaSeconds :type Float%20%28single-precision%29)))

(fn ConstructionScript)

(fn PlaceActors
  (bind _placeclasses (Variables|Default|GetPlaceClasses))
  ;[1 1 1] 少ない方に合わせて繰り返し
  (bind _output_get (Variables|Default|SetNumClasses (Utilities|Array|Length (Variables|Default|GetPlaceClasses))))
  (bind _output_get_2 (Variables|Default|SetNumTransforms (Utilities|Array|Length (Variables|Default|GetPlaceTransforms))))
  (bind _output_get_3 (Variables|Default|SetCount (Math|Integer|Min(Integer) _output_get _output_get_2)))
  (for _index (range 0 (- _output_get_3 1))
    ;[1 1 1] 問題なければクラスのコピーを対応Transformで配置
    (if (Utilities|Array|IsValidIndex _placeclasses _index)
      (bind _returnvalue (Game|SpawnActorfromClass (Utilities|Array|Get(acopy) _placeclasses _index) (Utilities|Array|Get(acopy) (Variables|Default|GetPlaceTransforms) _index) "Undefined" "MultiplyWithRoot" 0 0))
      (Utilities|Array|Add (Variables|Default|GetSpawnedActors) _returnvalue)
      (else
        ;[1 1 1] クラスが見つからなければエラーテキスト
        (Development|PrintString (Utilities|String|Append "Placement Error at index:" (Utilities|String|ToString(Integer) _index)))))))

(fn DestroyActors
  (bind _spawnedactors (Variables|Default|GetSpawnedActors))
  (for _array_element _spawnedactors
    (Actor|DestroyActor _array_element))
  (Utilities|Array|Clear _spawnedactors))