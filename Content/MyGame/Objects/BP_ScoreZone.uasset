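; BP_ScoreZone is a goal zone that awards points when a scorable object enters its box.
; On overlap, it reads the value through the BPI Scorable interface and adds it to the score in BP_FirstPersonGameMode.
; It then spawns an explosion, plays its sound midway between player and object, destroys the object and shakes the camera.
; A similar, disconnected scoring chain remains unused.
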(event OnComponentBeginOverlap(Box)
  (params (OverlappedComponent :type Primitive%20Component%20Object%20Reference) (OtherActor :type Actor%20Object%20Reference) (OtherComp :type Primitive%20Component%20Object%20Reference) (OtherBodyIndex :type Integer) (bFromSweep :type Boolean) (SweepResult :type Hit%20Result%20Structure%20%28by%20ref%29))
  (bind _returnvalue (Transformation|GetWorldLocation OtherComp))
  (if (Utilities|DoesObjectImplementInterface OtherActor "/Game/MyGame/Others/BPI＿Scorable.BPI＿Scorable_C")
    (bind _asbpi_scorable (Utilities|Casting|CastToBPI＿Scorable OtherActor))
    (bind _returnvalue_2 (Default|GetScoreValue _asbpi_scorable))
    (bind _asbp_first_person_game_mode (Utilities|Casting|CastToBP_FirstPersonGameMode (Game|GetGameMode)))
    (Default|AddScore _asbp_first_person_game_mode _returnvalue_2)
    (Effects|SpawnEmitteratLocation "/Game/StarterContent/Particles/P_Explosion.P_Explosion" _returnvalue "0, 0, 0" "3.000000,3.000000,3.000000")
    (Audio|PlaySoundatLocation "/Game/StarterContent/Audio/Explosion_Cue.Explosion_Cue" (/ (+ (Transformation|GetActorLocation (Game|GetPlayerCharacter 0)) _returnvalue) "2.000000,2.000000,2.000000") "0, 0, 0" 3.0 1.0 0.0 0 0 0 0)
    (Actor|DestroyActor OtherActor)
    (CameraShakes|StartCameraShake (Game|GetPlayerCameraManager 0) "/Game/MyGame/Others/BP_ScoreCameraShake.BP_ScoreCameraShake_C" 1.0 "CameraLocal" "0, 0, 0")))

(event EventBeginPlay)

(event EventTick
  (params (DeltaSeconds :type Float%20%28single-precision%29)))

(fn ConstructionScript)